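; PortalActivator is a key socket that takes a portal key from the player and helps reveal a linked Portal.
; On box overlap by a ThirdPersonCharacter, it tries to remove a key and, if successful, locks as activated and shows its hidden Key.
; The same attempt calls ShowPortal when the player's TotalPortalKeysCollected equals three.
; Highlight events toggle custom depth on the base and cutout meshes for a stencil outline.
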(event `self.ReceiveBeginPlay`
  (`SceneComponent.SetVisibility` (`self.Key`) false true))

(event `self.Box.OnComponentBeginOverlap`
  (params (OverlappedComponent :type "PrimitiveComponent Object Reference") (OtherActor :type "Actor Object Reference") (OtherComp :type "PrimitiveComponent Object Reference") (OtherBodyIndex :type Integer) (bFromSweep :type Boolean) (SweepResult :type "HitResult Structure (by ref)"))
  (bind _asthird_person_character (cast `/Game/ThirdPersonBP/Blueprints/ThirdPersonCharacter` OtherActor))
  (if (not (`self.isActivated`))
    (bind _haskey (`self.HandlePlayerPortalInteractions` _asthird_person_character))
    (if _haskey
      (set `self.isActivated` true)
      (`SceneComponent.SetVisibility` (`self.Key`) true true))))

(event `/Game/Blueprints/IHighlightable.StartHighlight`
  (bind _partsofmesh (`self.GetObjectMeshComponents`))
  (for _array_element _partsofmesh
    (`PrimitiveComponent.SetRenderCustomDepth` _array_element true)
    (`PrimitiveComponent.SetCustomDepthStencilValue` _array_element (`self.OutlineStencilDepth`))))

(event `/Game/Blueprints/IHighlightable.StopHighlight`
  (bind _partsofmesh (`self.GetObjectMeshComponents`))
  (for _array_element _partsofmesh
    (`PrimitiveComponent.SetRenderCustomDepth` _array_element false)))

(fn `GetObjectMeshComponents`
  (returns (PartsOfMesh :type "Array of PrimitiveComponent Object Reference"))
  (locals (Parts :type "Array of StaticMeshComponent Object Reference"))
  (return (`|MakeArray` (`self.Base`) (`self.Cutout1`) (`self.Cutout2`) (`self.Cutout3`) (`self.Cutout4`) (`self.Cutout5`) (`self.Cutout6`) (`self.Cutout7`) (`self.Cutout8`) :!type "PrimitiveComponent Object Reference")))

(fn `HandlePlayerPortalInteractions`
  (params (Player :type "/Game/ThirdPersonBP/Blueprints/ThirdPersonCharacter Object Reference"))
  (returns (hasKey :type Boolean))
  (locals (NewLocalVar_0 :type Boolean :default false))
  (bind _haskey (`/Game/ThirdPersonBP/Blueprints/ThirdPersonCharacter.RemovePortalKey` Player))
  (if (== (`/Game/ThirdPersonBP/Blueprints/ThirdPersonCharacter.TotalPortalKeysCollected` Player) 3)
    (`/Game/Blueprints/InsanePortal.Show Portal` (`self.Portal`)))
  (return _haskey))

(fn `UserConstructionScript`)