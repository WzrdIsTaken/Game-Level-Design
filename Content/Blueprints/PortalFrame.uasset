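; PortalFrame is a Blueprint for a portal frame built from four mesh pieces (bottom, top, left and right) that can be highlighted.
; StartHighlight enables custom depth rendering on each piece and writes the outline stencil value, and StopHighlight turns custom depth off.
; Both events get the pieces from GetObjectMeshComponents, so the whole frame highlights as one object.
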(event `/Game/Blueprints/IHighlightable.StartHighlight`
  (bind _newparam (`self.GetObjectMeshComponents`))
  (for _array_element _newparam
    (`PrimitiveComponent.SetRenderCustomDepth` _array_element true)
    (`PrimitiveComponent.SetCustomDepthStencilValue` _array_element (`self.OutlineStencilDepth`))))

(event `/Game/Blueprints/IHighlightable.StopHighlight`
  (bind _newparam (`self.GetObjectMeshComponents`))
  (for _array_element _newparam
    (`PrimitiveComponent.SetRenderCustomDepth` _array_element false)))

(fn `GetObjectMeshComponents`
  (returns (NewParam :type "Array of PrimitiveComponent Object Reference"))
  (return (`|MakeArray` (`self.Bot`) (`self.Top`) (`self.Left`) (`self.Right`) :!type "PrimitiveComponent Object Reference")))

(fn `UserConstructionScript`)