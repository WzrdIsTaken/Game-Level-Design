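; One-way portal actor that teleports a ThirdPersonCharacter from an entrance to the exit portal sharing its PortalIndex.
; It starts with collision off, and ActivatePortal toggles visibility and enables collision.
; On hit, an active entrance searches all Portal actors, moves the character to the exit's ExitReference and destroys that exit; the reverse-direction branch is unreachable.
; The construction script applies the editable portal transform and exit location.
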(event `self.ReceiveBeginPlay`
  (`SceneComponent.ToggleVisibility` (`self.Portal`) false)
  (`self.SetActorEnableCollision` false))

(event `ActivatePortal`
  (set `self.isActive` true)
  (`SceneComponent.ToggleVisibility` (`self.Portal`) false)
  (`self.SetActorEnableCollision` true))

(event `self.ReceiveHit`
  (params (MyComp :type "PrimitiveComponent Object Reference") (Other :type "Actor Object Reference") (OtherComp :type "PrimitiveComponent Object Reference") (bSelfMoved :type Boolean) (HitLocation :type "Vector Structure") (HitNormal :type "Vector Structure") (NormalImpulse :type "Vector Structure") (Hit :type "HitResult Structure (by ref)"))
  (if (and (`self.isActive`) (`self.isEnterance`))
    (bind _asthird_person_character (cast `/Game/ThirdPersonBP/Blueprints/ThirdPersonCharacter` Other))
    (if (`self.isEnterance`)
      (bind _outactors (`GameplayStatics.GetAllActorsOfClass` "Portal_C"))
      (for _array_element _outactors
        (if (and (== (`/Game/Blueprints/Portal.PortalIndex` _array_element) (`self.PortalIndex`)) (not (`/Game/Blueprints/Portal.isEnterance` _array_element)))
          (break)))
      (`self.K2_SetActorLocation` _asthird_person_character (`SceneComponent.K2_GetComponentLocation` (`/Game/Blueprints/Portal.Exit Reference` _array_element)) false false)
      (`self.K2_DestroyActor` _array_element)
      (else
        (bind _outactors_2 (`GameplayStatics.GetAllActorsOfClass` "Portal_C"))
        (for _array_element_2 _outactors_2
          (if (and (== (`/Game/Blueprints/Portal.PortalIndex` _array_element_2) (`self.PortalIndex`)) (and (not (`self.isEnterance`)) (`/Game/Blueprints/Portal.isEnterance` _array_element_2)))
            (break)))
        (`self.K2_SetActorLocation` _asthird_person_character (`SceneComponent.K2_GetComponentLocation` (`/Game/Blueprints/Portal.Exit Reference` _array_element_2)) false false)))))

(fn `UserConstructionScript`
  (`SceneComponent.K2_SetRelativeTransform` (`self.Portal`) (`self.PortalTransform`) false false)
  (`SceneComponent.K2_SetRelativeLocation` (`self.Exit Reference`) (`self.ExitLocation`) false false))