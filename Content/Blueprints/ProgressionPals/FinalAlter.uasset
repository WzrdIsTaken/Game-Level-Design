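; Final altar actor that ends the game in victory when a player character with Divine Guidance overlaps its box.
; The ending destroys the player's capsule, stops the world darkening, switches to a final camera and plays a level sequence.
; After a hard-coded delay matching the sequence length, it shows the win widget and allows restarting.
; Separate highlight events toggle an outline on the mesh through custom depth stencil.
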(event `self.Box.OnComponentBeginOverlap`
  (params (OverlappedComponent :type "PrimitiveComponent Object Reference") (OtherActor :type "Actor Object Reference") (OtherComp :type "PrimitiveComponent Object Reference") (OtherBodyIndex :type Integer) (bFromSweep :type Boolean) (SweepResult :type "HitResult Structure (by ref)"))
  ;[1 1 1] Collision
  (bind _asthird_person_character (cast `/Game/Blueprints/ThirdPersonCharacter` OtherActor))
  (if (`/Game/Blueprints/ThirdPersonCharacter.hasDivineGuidance` _asthird_person_character)
    (`self.StartFinalCutscene`)))

(event `StartFinalCutscene`
  ;[1 1 1] Cutscene / end state
  (bind _asthird_person_character (cast `/Game/Blueprints/ThirdPersonCharacter` (`GameplayStatics.GetPlayerCharacter` 0)))
  (bind _output_get (set `self.Player` _asthird_person_character))
  (`/Game/Blueprints/ThirdPersonCharacter.DestroyCapsuleComponent` _output_get)
  (`/Game/Blueprints/ProgressionPals/FinalDarkenSequence.StopWorldDarken` (`self.DarkenWorld`))
  (`PlayerController.SetViewTargetWithBlend` (`GameplayStatics.GetPlayerController` 0) (`self.FinalCamera`) 0.0 "VTBlend_Linear" 0.0 false)
  (`MovieSceneSequencePlayer.Play` (`LevelSequenceActor.SequencePlayer` (`self.FinalCutsceneSequence`)))
  (`KismetSystemLibrary.Delay` 10.0) ; 10 = length of sequence
  (bind _returnvalue (`|CreateWidget` "/Game/UI/YouWinWidget.YouWinWidget_C"))
  (`UserWidget.AddToViewport` _returnvalue 0)
  (`/Game/Blueprints/ThirdPersonCharacter.SetCanRestart` (`self.Player`)))

(event `/Game/Blueprints/IHighlightable.StartHighlight`
  (bind _staticmesh (`self.StaticMesh`))
  ;[1 1 1] Hightlight
  (`PrimitiveComponent.SetRenderCustomDepth` _staticmesh true)
  (`PrimitiveComponent.SetCustomDepthStencilValue` _staticmesh (`self.OutlineStencilDepth`)))

(event `/Game/Blueprints/IHighlightable.StopHighlight`
  ;[1 1 1] Hightlight
  (`PrimitiveComponent.SetRenderCustomDepth` (`self.StaticMesh`) false))

(fn `UserConstructionScript`)