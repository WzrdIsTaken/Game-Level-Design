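; Trigger actor for a final darkening sequence that blacks out the player's view and kills them.
; The first ThirdPersonCharacter overlap of its Box starts the darkening, and Tick raises a time-scaled darkness value into the player's SetBlackClip until it passes the maximum and calls Die.
; StopWorldDarken fades the value back toward zero but is not called here.
; The DarkenState names run opposite to the value: DecreasingDarkness raises it, IncreasingDarkness lowers it.
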(event `self.Box.OnComponentBeginOverlap`
  (params (OverlappedComponent :type "PrimitiveComponent Object Reference") (OtherActor :type "Actor Object Reference") (OtherComp :type "PrimitiveComponent Object Reference") (OtherBodyIndex :type Integer) (bFromSweep :type Boolean) (SweepResult :type "HitResult Structure (by ref)"))
  ;[1 1 1] Collision
  (cast `/Game/Blueprints/ThirdPersonCharacter` OtherActor)
  (if (not (`self.hasCollided`))
    (set `self.hasCollided` true)
    (`self.StartWorldDarken`)))

(event `StartWorldDarken`
  ;[1 1 1] Events
  (set `self.DarkenState` "NewEnumerator2"))

(event `StopWorldDarken`
  ;[1 1 1] Events
  (set `self.DarkenState` "NewEnumerator1"))

(event `self.ReceiveTick`
  (params (DeltaSeconds :type "Float (single-precision)"))
  (bind _returnvalue (`GameplayStatics.GetWorldDeltaSeconds`))
  (bind _darknessvalue (`self.DarknessValue`))
  ;[1 1 1] Darken World
  (switch `/Game/Blueprints/ProgressionPals/FinalDarkenState` (`self.DarkenState`)
    (:`NewEnumerator1`
      (bind _output_get (set `self.DarknessValue` (- _darknessvalue (* _returnvalue (`self.DarknessDecreaseRate`)))))
      (if (< _output_get 0.0)
        (set `self.DarkenState` "NewEnumerator0")
        (else
          (`/Game/Blueprints/ThirdPersonCharacter.SetBlackClip` (`self.Player`) (`self.DarknessValue`) :!label _label))))
    (:`NewEnumerator2`
      (bind _output_get_2 (set `self.DarknessValue` (+ _darknessvalue (* (`self.DarknessIncreaseRate`) _returnvalue))))
      (if (> _output_get_2 (`self.MaxDarknessValue`))
        (set `self.DarkenState` "NewEnumerator0")
        (`/Game/Blueprints/ThirdPersonCharacter.Die` (`self.Player`) true)
        (else
          (goto _label))))))

(fn `UserConstructionScript`)