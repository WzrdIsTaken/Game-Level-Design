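; Door actor, named for a traps corridor, that opens once for a ThirdPersonCharacter with divine guidance.
; Overlapping its box checks that flag, then latches HasOpened and raises the door component with an eased MoveComponentTo over OpenTime.
; StartHighlight and StopHighlight toggle custom depth on door and handle, using a stencil value for outlining.
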(event `self.Box.OnComponentBeginOverlap`
  (params (OverlappedComponent :type "PrimitiveComponent Object Reference") (OtherActor :type "Actor Object Reference") (OtherComp :type "PrimitiveComponent Object Reference") (OtherBodyIndex :type Integer) (bFromSweep :type Boolean) (SweepResult :type "HitResult Structure (by ref)"))
  (bind _asthird_person_character (cast `/Game/ThirdPersonBP/Blueprints/ThirdPersonCharacter` OtherActor))
  (if (and (`/Game/ThirdPersonBP/Blueprints/ThirdPersonCharacter.hasDivineGuidance` _asthird_person_character) (not (`self.hasOpened`)))
    (set `self.hasOpened` true)
    (`KismetSystemLibrary.MoveComponentTo` (`self.Door`) (0.0 0.0 1000.0) (struct) true true (`self.OpenTime`))))

(event `/Game/Blueprints/IHighlightable.StartHighlight`
  (`PrimitiveComponent.SetRenderCustomDepth` (`self.Door`) true)
  (`PrimitiveComponent.SetRenderCustomDepth` (`self.Handle`) true)
  (`PrimitiveComponent.SetCustomDepthStencilValue` (`self.Handle`) (`self.OutlineStencilValue`))
  (`PrimitiveComponent.SetCustomDepthStencilValue` (`self.Door`) (`self.OutlineStencilValue`)))

(event `/Game/Blueprints/IHighlightable.StopHighlight`
  (`PrimitiveComponent.SetRenderCustomDepth` (`self.Door`) false)
  (`PrimitiveComponent.SetRenderCustomDepth` (`self.Handle`) false))

(fn `UserConstructionScript`)