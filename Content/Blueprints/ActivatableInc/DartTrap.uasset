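; DartTrap is an activatable trap that fires a Dart actor when switched on.
; When Activate receives a true IsActive, it spawns one Dart at the ShootPoint component's world transform, with the trap as owner.
; Deactivation does nothing, and the overlap and tick events are disabled stubs.
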(event `/Game/Blueprints/ActivatableInc/IActivatable.Activate`
  (params (isActive :type Boolean))
  (if isActive
    (`|SpawnActorFromClass` "/Game/Blueprints/ActivatableInc/Dart.Dart_C" (`SceneComponent.K2_GetComponentToWorld` (`self.ShootPoint`)) "Undefined" "OverrideRootScale" self null)))

(fn `UserConstructionScript`
  (`parent.UserConstructionScript`))