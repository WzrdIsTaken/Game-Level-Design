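; MovingWall is a trap or obstacle wall that starts moving when a ThirdPersonCharacter overlaps its Collider.
; A one-shot flag guards the sequence, so later overlaps are ignored.
; MoveComponentTo first shifts the Wall to a lowered relative position over MoveDownTime.
; It then chains into an eased move to a point far along local Y at zero height, travelling down the corridor over MoveAlongTime.
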(event `self.Collider.OnComponentBeginOverlap`
  (params (OverlappedComponent :type "PrimitiveComponent Object Reference") (OtherActor :type "Actor Object Reference") (OtherComp :type "PrimitiveComponent Object Reference") (OtherBodyIndex :type Integer) (bFromSweep :type Boolean) (SweepResult :type "HitResult Structure (by ref)"))
  ;[1 1 1] Collision
  (cast `/Game/Blueprints/ThirdPersonCharacter` OtherActor)
  (`self.MoveDown`))

(event `MoveDown`
  ;[1 1 1] Move Down
  (if (not (`self.hasStartedMoving`))
    (set `self.hasStartedMoving` true)
    (`KismetSystemLibrary.MoveComponentTo` (`self.Wall`) (0.0 0.0 -100.0) (struct) false false (`self.MoveDownTime`))
    (`self.MoveForward`)))

(event `MoveForward`
  ;[1 1 1] Move forward (down corridoor)
  (`KismetSystemLibrary.MoveComponentTo` (`self.Wall`) (0.0 11250.0 0.0) (struct) true true (`self.MoveAlongTime`)))

(fn `UserConstructionScript`)