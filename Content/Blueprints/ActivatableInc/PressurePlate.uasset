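; Pressure plate that sinks when a ThirdPersonCharacter steps on it and activates its linked dart traps.
; Trigger overlaps drive the Push timeline that moves the plate, reversing it once nothing overlaps.
; Traps receive ActivateMessage immediately on the first press only, through a bug-workaround function replacing the deprecated timeline-finished activation.
; Highlight events toggle a custom-depth stencil outline on the plate when traps are linked.
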(event `self.Trigger.OnComponentBeginOverlap`
  (params (OverlappedComponent :type "PrimitiveComponent Object Reference") (OtherActor :type "Actor Object Reference") (OtherComp :type "PrimitiveComponent Object Reference") (OtherBodyIndex :type Integer) (bFromSweep :type Boolean) (SweepResult :type "HitResult Structure (by ref)"))
  ;[1 1 1] Collision
  (cast `/Game/Blueprints/ThirdPersonCharacter` OtherActor)
  (if (not (`self.isPressed`))
    (set `self.isPressed` true)
    (`self.BotActivationLogicBecauseBug`)
    (bind (_direction _push) (`Timeline|Push` :!label _label)
      (:`Update`
        (`SceneComponent.K2_SetRelativeLocation` (`self.Plate`) (`KismetMathLibrary.MakeVector` 0.0 0.0 _push) false false)))))

(event `self.Trigger.OnComponentEndOverlap`
  (params (OverlappedComponent :type "PrimitiveComponent Object Reference") (OtherActor :type "Actor Object Reference") (OtherComp :type "PrimitiveComponent Object Reference") (OtherBodyIndex :type Integer))
  ;[1 1 1] Collision
  (cast `/Game/Blueprints/ThirdPersonCharacter` OtherActor)
  (if (not (`KismetArrayLibrary.Array_IsValidIndex` (`PrimitiveComponent.GetOverlappingActors` (`self.Trigger`) null)))
    (set `self.isPressed` false)
    (goto _label :!via `Reverse`)))

(event `/Game/Blueprints/IHighlightable.StartHighlight`
  (bind _plate (`self.Plate`))
  ;[1 1 1] Highlight
  (if (!= (`KismetArrayLibrary.Array_Length` (`self.DartTraps`)) 0)
    (`PrimitiveComponent.SetRenderCustomDepth` _plate true)
    (`PrimitiveComponent.SetCustomDepthStencilValue` _plate (`self.OutlineStencilValue`))))

(event `/Game/Blueprints/IHighlightable.StopHighlight`
  ;[1 1 1] Highlight
  (if (!= (`KismetArrayLibrary.Array_Length` (`self.DartTraps`)) 0)
    (`PrimitiveComponent.SetRenderCustomDepth` (`self.Plate`) false)))

(fn `BotActivationLogicBecauseBug`
  (if (and (not (== (`KismetArrayLibrary.Array_Length` (`self.DartTraps`)) 0)) (not (`self.hasActivated`)))
    (set `self.hasActivated` true)
    (for _array_element (`self.DartTraps`)
      (message `/Game/Blueprints/ActivatableInc/IActivatable.Activate` _array_element true))))

(fn `UserConstructionScript`)