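; PortalKey is a pickup actor that the player collects by walking into it.
; When the third-person character overlaps its collider, it adds a portal key to that character and destroys itself.
; Highlight events toggle a custom-depth stencil outline on the key mesh.
; An older, disconnected path that counted keys through the game mode and showed the portal is left unused.
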(event `self.Collider.OnComponentBeginOverlap`
  (params (OverlappedComponent :type "PrimitiveComponent Object Reference") (OtherActor :type "Actor Object Reference") (OtherComp :type "PrimitiveComponent Object Reference") (OtherBodyIndex :type Integer) (bFromSweep :type Boolean) (SweepResult :type "HitResult Structure (by ref)"))
  ;[1 1 1] Collision
  (bind _asthird_person_character (cast `/Game/Blueprints/ThirdPersonCharacter` OtherActor))
  (`/Game/Blueprints/ThirdPersonCharacter.AddPortalKey` _asthird_person_character)
  (`self.K2_DestroyActor`))

(event `/Game/Blueprints/IHighlightable.StartHighlight`
  (bind _key (`self.Key`))
  ;[1 1 1] Highlight
  (`PrimitiveComponent.SetRenderCustomDepth` _key true)
  (`PrimitiveComponent.SetCustomDepthStencilValue` _key (`self.OutlineStencilValue`)))

(event `/Game/Blueprints/IHighlightable.StopHighlight`
  ;[1 1 1] Highlight
  (`PrimitiveComponent.SetRenderCustomDepth` (`self.Key`) false))

(fn `UserConstructionScript`)