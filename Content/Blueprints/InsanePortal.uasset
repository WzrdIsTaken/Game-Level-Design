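; InsanePortal is a portal actor that teleports an overlapping ThirdPersonCharacter to its Target portal, keeping the player's control rotation.
; It hides the Target before a briefly delayed teleport, preventing bounce-back; leaving a portal's capsule reshows it unless one-way.
; A cube scene capture runs at construction, then once or every frame during play.
; The Map cubemap feeds a dynamic material driving the portal's Niagara effect.
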(event `self.ReceiveBeginPlay`
  (if (`self.CaptureEveryFrame`)
    (set `SceneCaptureComponent.bCaptureEveryFrame` true (`self.SceneCaptureComponentCube`))
    (else
      (`SceneCaptureComponentCube.CaptureScene` (`self.SceneCaptureComponentCube`))))
  (if (`self.startHidden`)
    (`self.HidePortal`)))

(event `self.Capsule.OnComponentBeginOverlap`
  (params (OverlappedComponent :type "PrimitiveComponent Object Reference") (OtherActor :type "Actor Object Reference") (OtherComp :type "PrimitiveComponent Object Reference") (OtherBodyIndex :type Integer) (bFromSweep :type Boolean) (SweepResult :type "HitResult Structure (by ref)"))
  (bind _target (`self.Target`))
  (bind _asthird_person_character (cast `/Game/ThirdPersonBP/Blueprints/ThirdPersonCharacter` OtherActor))
  (if (`self.canPort`)
    (set `self.Player` _asthird_person_character)
    (`self.HidePortal` _target)
    (`KismetSystemLibrary.Delay` 0.1)
    (`/Game/ThirdPersonBP/Blueprints/ThirdPersonCharacter.PortalTo` (`self.Player`) (`SceneComponent.K2_GetComponentLocation` (`/Game/Blueprints/InsanePortal.Capsule` _target)) (`Controller.GetControlRotation` (`GameplayStatics.GetPlayerController` 0)))))

(event `self.Capsule.OnComponentEndOverlap`
  (params (OverlappedComponent :type "PrimitiveComponent Object Reference") (OtherActor :type "Actor Object Reference") (OtherComp :type "PrimitiveComponent Object Reference") (OtherBodyIndex :type Integer))
  (cast `/Game/ThirdPersonBP/Blueprints/ThirdPersonCharacter` OtherActor)
  (if (not (`self.isOneWay`))
    (`self.Show Portal`)))

(event `Show Portal`
  (`ActorComponent.SetActive` (`self.InsanePortalEffect`) true true)
  (set `self.canPort` true))

(event `HidePortal`
  (`ActorComponent.Deactivate` (`self.InsanePortalEffect`))
  (set `self.canPort` false))

(fn `UserConstructionScript`
  (`SceneCaptureComponentCube.CaptureScene` (`self.SceneCaptureComponentCube`))
  (bind _returnvalue (`KismetMaterialLibrary.CreateDynamicMaterialInstance` (`self.MaterialInstance`)))
  (`MaterialInstanceDynamic.SetTextureParameterValue` _returnvalue "CubeMap" (`self.Map`))
  (`NiagaraComponent.SetVariableMaterial` (`self.InsanePortalEffect`) "MIC" _returnvalue))