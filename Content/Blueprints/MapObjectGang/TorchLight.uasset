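; Torch light actor that makes its point light flicker by continually drifting between random intensities.
; BeginPlay picks a random flicker speed and target brightness and sets a random starting intensity.
; Tick uses FInterpTo to ease intensity toward the target, rolling a new speed and target once they match exactly.
; The MinFlickerTime and MaxFlickerTime range feeds the interpolation speed, so larger values flicker faster.
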(event `self.ReceiveBeginPlay`
  (`|ExecutionSequence`
    (:`then_0`
      (`self.SetFlickerSpeed`))
    (:`then_1`
      (bind _brightness (`self.SetTargetBrightness`))
      (`LightComponent.SetIntensity` (`self.PointLightComponent`) _brightness))))

(event `self.ReceiveTick`
  (params (DeltaSeconds :type "Float (single-precision)"))
  (`|ExecutionSequence`
    (:`then_0`
      (if (== (`LightComponentBase.Intensity` (`self.PointLightComponent`)) (`self.TargetBrightness`))
        (`self.SetFlickerSpeed`)
        (`self.SetTargetBrightness`)))
    (:`then_1`
      (`LightComponent.SetIntensity` (`self.PointLightComponent`) (`KismetMathLibrary.FInterpTo` (`LightComponentBase.Intensity` (`self.PointLightComponent`)) (`self.TargetBrightness`) DeltaSeconds (`self.FlickerSpeed`))))))

(fn `SetFlickerSpeed`
  (set `self.FlickerSpeed` (`KismetMathLibrary.RandomFloatInRange` (`self.MinFlickerTime`) (`self.MaxFlickerTime`))))

(fn `SetTargetBrightness`
  (returns (Brightness :type "Float (double-precision)"))
  (bind _returnvalue (`KismetMathLibrary.RandomFloatInRange` (`self.MinBrightness`) (`self.MaxBrightness`)))
  (set `self.TargetBrightness` _returnvalue)
  (return _returnvalue))

(fn `UserConstructionScript`)