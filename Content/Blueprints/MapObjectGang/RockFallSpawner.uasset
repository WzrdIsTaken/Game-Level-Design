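; Rock fall spawner actor that holds a single hidden rock, DropCube, ready to drop into the map when triggered.
; On BeginPlay it randomizes the rock's scale, rotation and mass override, then hides it.
; The SpawnRock event makes that prepared rock visible and turns on physics simulation, so no new actor is spawned at drop time.
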(event `self.ReceiveBeginPlay`
  (bind _returnvalue (`KismetMathLibrary.RandomFloat`))
  ;[1 1 1] Create rock ready to be activated
  (`SceneComponent.SetWorldScale3D` (`self.DropCube`) (`KismetMathLibrary.VLerp` (0.1 0.1 0.1) (0.25 0.25 0.25) _returnvalue))
  (`SceneComponent.K2_SetWorldRotation` (`self.DropCube`) (`KismetMathLibrary.RLerp` (struct) (struct :`Pitch` 360.0 :`Yaw` 360.0 :`Roll` 360.0) _returnvalue) false false)
  (`PrimitiveComponent.SetMassOverrideInKg` (`self.DropCube`) "None" (`KismetMathLibrary.RandomFloatInRange` 1000.0 2000.0) true)
  (`SceneComponent.SetVisibility` (`self.DropCube`) false false))

(event `SpawnRock`
  ;[1 1 1] Activate rock
  (`SceneComponent.SetVisibility` (`self.DropCube`) true false)
  (`PrimitiveComponent.SetSimulatePhysics` (`self.DropCube`) true))

(fn `UserConstructionScript`)