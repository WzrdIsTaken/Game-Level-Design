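; Rock actor that stays hidden until DropRock reveals it and lets it fall as a physics object.
; On BeginPlay it randomizes the static mesh's uniform scale, rotation and mass override for variety, then hides the mesh.
; The DropRock event makes the mesh visible and enables physics simulation; nothing in this Blueprint calls that event itself.
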(event `self.ReceiveBeginPlay`
  (bind _returnvalue (`KismetMathLibrary.RandomFloat`))
  ;[1 1 1] Setup Rock
  (`SceneComponent.SetWorldScale3D` (`self.StaticMesh`) (`KismetMathLibrary.VLerp` (0.1 0.1 0.1) (0.25 0.25 0.25) _returnvalue))
  (`SceneComponent.K2_SetWorldRotation` (`self.StaticMesh`) (`KismetMathLibrary.RLerp` (struct) (struct :`Pitch` 360.0 :`Yaw` 360.0 :`Roll` 360.0) _returnvalue) false false)
  (`PrimitiveComponent.SetMassOverrideInKg` (`self.StaticMesh`) "None" (`KismetMathLibrary.RandomFloatInRange` 1000.0 2000.0) true)
  (`SceneComponent.SetVisibility` (`self.StaticMesh`) false false))

(event `DropRock`
  ;[1 1 1] Activate rock
  (`SceneComponent.SetVisibility` (`self.StaticMesh`) true false)
  (`PrimitiveComponent.SetSimulatePhysics` (`self.StaticMesh`) true))

(fn `UserConstructionScript`)