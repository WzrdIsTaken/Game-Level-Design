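; Floating platform Blueprint that moves back and forth between its placed location and a target location using an InterpToMovement component.
; The construction script builds two absolute control points from the actor's location and TargetLocation.
; It also picks a random travel duration between MinDuration and MaxDuration, so the random element is the timing of each platform, not its endpoints.
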(fn `UserConstructionScript`
  (bind _interptomovement (`self.InterpToMovement`))
  (set `InterpToMovementComponent.ControlPoints` (`|MakeArray` (make `InterpControlPoint` (`self.K2_GetActorLocation`) false) (make `InterpControlPoint` (`self.TargetLocation`) false)) _interptomovement)
  (set `InterpToMovementComponent.Duration` (`KismetMathLibrary.RandomFloatInRange` (`self.MinDuration`) (`self.MaxDuration`)) _interptomovement))